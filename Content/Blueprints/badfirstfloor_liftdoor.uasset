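; First-floor lift door Blueprint that slides two door meshes open and closed on trigger overlaps.
; Doorbox and Leveltrigger each play their own timeline after a delay on entry and reverse it after leaving.
; A LevelTrigger flag, set by Leveltrigger and cleared on either exit, blocks Doorbox from starting its animation.
; Timelines add offsets to positions cached at BeginPlay, except Doorbox offsets the first door from its position sampled after the delay.
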(event `self.ReceiveBeginPlay`
  (set `self.Doorlocation1` (`SceneComponent.K2_GetComponentLocation` (`self.Lift_Door2_StaticMesh`)))
  (set `self.doorlocation2` (`SceneComponent.K2_GetComponentLocation` (`self.Lift_Door3_StaticMesh`)))
  (set `self.level_trigger` false))

(event `self.doorbox.OnComponentBeginOverlap`
  (params (OverlappedComponent :type "PrimitiveComponent Object Reference") (OtherActor :type "Actor Object Reference") (OtherComp :type "PrimitiveComponent Object Reference") (OtherBodyIndex :type Integer) (bFromSweep :type Boolean) (SweepResult :type "HitResult Structure (by ref)"))
  (if (not (`self.level_trigger`))
    (`KismetSystemLibrary.Delay` 2.0)
    (set `self.doorclose` (`SceneComponent.K2_GetComponentLocation` (`self.Lift_Door2_StaticMesh`)))
    (bind (_direction _newtrack_0 _newtrack2) (`Timeline|floordoors` :!via `PlayFromStart` :!label _label)
      (:`Update`
        (`SceneComponent.K2_SetWorldLocation` (`self.Lift_Door2_StaticMesh`) (+ _newtrack_0 (`self.doorclose`)) false false)
        (`SceneComponent.K2_SetWorldLocation` (`self.Lift_Door3_StaticMesh`) (+ _newtrack2 (`self.doorlocation2`)) false false)))))

(event `self.doorbox.OnComponentEndOverlap`
  (params (OverlappedComponent :type "PrimitiveComponent Object Reference") (OtherActor :type "Actor Object Reference") (OtherComp :type "PrimitiveComponent Object Reference") (OtherBodyIndex :type Integer))
  (set `self.level_trigger` false)
  (`KismetSystemLibrary.Delay` 2.0)
  (goto _label :!via `Reverse`))

(event `self.leveltrigger.OnComponentBeginOverlap`
  (params (OverlappedComponent :type "PrimitiveComponent Object Reference") (OtherActor :type "Actor Object Reference") (OtherComp :type "PrimitiveComponent Object Reference") (OtherBodyIndex :type Integer) (bFromSweep :type Boolean) (SweepResult :type "HitResult Structure (by ref)"))
  (set `self.level_trigger` true)
  (`KismetSystemLibrary.Delay` 2.0)
  (set `self.doorclose` (`SceneComponent.K2_GetComponentLocation` (`self.Lift_Door2_StaticMesh`)))
  (bind (_direction _newtrack_0 _newtrack2) (`Timeline|Timeline_0` :!via `PlayFromStart` :!label _label_2)
    (:`Update`
      (`SceneComponent.K2_SetWorldLocation` (`self.Lift_Door2_StaticMesh`) (+ _newtrack_0 (`self.Doorlocation1`)) false false)
      (`SceneComponent.K2_SetWorldLocation` (`self.Lift_Door3_StaticMesh`) (+ _newtrack2 (`self.doorlocation2`)) false false))))

(event `self.leveltrigger.OnComponentEndOverlap`
  (params (OverlappedComponent :type "PrimitiveComponent Object Reference") (OtherActor :type "Actor Object Reference") (OtherComp :type "PrimitiveComponent Object Reference") (OtherBodyIndex :type Integer))
  (set `self.level_trigger` false)
  (`KismetSystemLibrary.Delay` 2.0)
  (set `self.doorclose` (`SceneComponent.K2_GetComponentLocation` (`self.Lift_Door2_StaticMesh`)))
  (goto _label_2 :!via `Reverse`))

(fn `UserConstructionScript`)