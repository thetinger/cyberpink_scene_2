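; Actor Blueprint for carrying physics objects with a Physics Handle while E is held, releasing on key up.
; Each tick while active, it moves the handle target along the control rotation's forward vector, scaled by OtherItemLocation, and matches that rotation.
; No trace or grab call appears in the graph.
; Both mouse wheel directions increase PickupDistance, since down subtracts a negative, and the target calculation never reads that variable.
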(event `self.ReceiveTick`
  (params (DeltaSeconds :type "Float (single-precision)"))
  (if (`self.Physics Handle Active`)
    (set `self.Handle Location` (+ (+ (`self.K2_GetActorLocation`) (* (`KismetMathLibrary.GetForwardVector` (`Pawn.GetControlRotation`)) (`self.Other Item Location`))) (0.0 0.0 0.0)))
    (`PhysicsHandleComponent.SetTargetLocationAndRotation` (`self.PhysicsHandle`) (`self.Handle Location`) (`Pawn.GetControlRotation`))))

(event `Key|E`
  (params (Key :type "Key Structure" :default "AnyKey"))
  (:`Pressed`
    (set `self.Physics Handle Active` true))
  (:`Released`
    (set `self.Physics Handle Active` false)
    (`PhysicsHandleComponent.ReleaseComponent` (`self.PhysicsHandle`))))

(event `Key|MouseScrollUp`
  (params (Key :type "Key Structure" :default "AnyKey"))
  (:`Pressed`
    (set `self.Pickup Distance` (+ (`self.Pickup Distance`) 25.0))))

(event `Key|MouseScrollDown`
  (params (Key :type "Key Structure" :default "AnyKey"))
  (:`Pressed`
    (set `self.Pickup Distance` (- (`self.Pickup Distance`) -25.0))))

(fn `UserConstructionScript`)