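; First-floor lift door actor that opens and closes its landing doors in step with the lift's own doors.
; An opendoors event or a Leveltrigger overlap finds the first Lift_blueprint, opens its doors and plays the Floordoors timeline.
; The timeline offsets the two door meshes from world positions cached at BeginPlay.
; A Closelift overlap closes the lift's doors and reverses the timeline.
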(event `self.ReceiveBeginPlay`
  (set `self.Doorlocation1` (`SceneComponent.K2_GetComponentLocation` (`self.Lift_Door2_StaticMesh`)))
  (set `self.doorlocation2` (`SceneComponent.K2_GetComponentLocation` (`self.Lift_Door3_StaticMesh`)))
  (set `self.Door Open` false))

(event `opendoors`
  (bind _outactors (`GameplayStatics.GetAllActorsOfClass` "/Game/Blueprints/Lift_blueprint.Lift_blueprint_C"))
  (`/Game/Blueprints/Lift_blueprint.openliftdoors` (`KismetArrayLibrary.Array_Get` _outactors))
  (bind (_direction _newtrack_0 _newtrack2) (`Timeline|floordoors` :!label _label)
    (:`Update`
      (`SceneComponent.K2_SetWorldLocation` (`self.Lift_Door2_StaticMesh`) (+ _newtrack_0 (`self.Doorlocation1`)) false false)
      (`SceneComponent.K2_SetWorldLocation` (`self.Lift_Door3_StaticMesh`) (+ _newtrack2 (`self.doorlocation2`)) false false))))

(event `self.closelift.OnComponentBeginOverlap`
  (params (OverlappedComponent :type "PrimitiveComponent Object Reference") (OtherActor :type "Actor Object Reference") (OtherComp :type "PrimitiveComponent Object Reference") (OtherBodyIndex :type Integer) (bFromSweep :type Boolean) (SweepResult :type "HitResult Structure (by ref)"))
  (bind _outactors (`GameplayStatics.GetAllActorsOfClass` "/Game/Blueprints/Lift_blueprint.Lift_blueprint_C"))
  (`/Game/Blueprints/Lift_blueprint.closeliftdoors` (`KismetArrayLibrary.Array_Get` _outactors))
  (goto _label :!via `Reverse`))

(event `self.leveltrigger.OnComponentBeginOverlap`
  (params (OverlappedComponent :type "PrimitiveComponent Object Reference") (OtherActor :type "Actor Object Reference") (OtherComp :type "PrimitiveComponent Object Reference") (OtherBodyIndex :type Integer) (bFromSweep :type Boolean) (SweepResult :type "HitResult Structure (by ref)"))
  (bind _outactors (`GameplayStatics.GetAllActorsOfClass` "/Game/Blueprints/Lift_blueprint.Lift_blueprint_C"))
  (`/Game/Blueprints/Lift_blueprint.openliftdoors` (`KismetArrayLibrary.Array_Get` _outactors))
  (goto _label))

(fn `UserConstructionScript`)