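; Elevator Blueprint that moves a lift one storey up or down when Lookingat receives its Up or Down component.
; MoveComponentTo eases the mesh between floors within height limits, gated by Ismovement and Doorstop flags.
; Open and close events play or reverse a timeline offsetting two door meshes, clearing Doorstop until the timeline updates.
; Trigger overlap events are empty, and the code opening Groundfloor_liftdoor actors is unconnected.
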(event `/Game/Blueprints/Playerclickinterface.LookingAt`
  (params (component :type "ActorComponent Object Reference"))
  (bind _staticmeshcomponent (`self.StaticMeshComponent`))
  (bind _staticmeshcomponent_2 (`self.StaticMeshComponent`))
  (bind (_returnvalue_x _returnvalue_y _returnvalue_z) (`KismetMathLibrary.BreakVector` (`SceneComponent.K2_GetComponentLocation` _staticmeshcomponent)))
  (bind (_returnvalue_x_2 _returnvalue_y_2 _returnvalue_z_2) (`KismetMathLibrary.BreakVector` (`SceneComponent.K2_GetComponentLocation` _staticmeshcomponent_2)))
  (if (`self.ismovement`)
    _
    (elif (`self.doorstop`)
      (if (== component (`self.Up`))
        (if (< (`self.current height`) (`self.max height`))
          (set `self.ismovement` true)
          (`KismetSystemLibrary.MoveComponentTo` _staticmeshcomponent_2 (`KismetMathLibrary.MakeVector` _returnvalue_x_2 _returnvalue_y_2 (+ _returnvalue_z_2 (`self.story height`))) (`SceneComponent.K2_GetComponentRotation` _staticmeshcomponent_2) true true (`self.elevator speed`))
          (set `self.current height` (+ (`self.current height`) (`self.story height`)))
          (set `self.ismovement` false))
        (elif (== component (`self.down`))
          (if (> (`self.current height`) (`self.min height`))
            (set `self.ismovement` true)
            (`KismetSystemLibrary.MoveComponentTo` _staticmeshcomponent (`KismetMathLibrary.MakeVector` _returnvalue_x _returnvalue_y (- _returnvalue_z (`self.story height`))) (`SceneComponent.K2_GetComponentRotation` _staticmeshcomponent) true true (`self.elevator speed`))
            (set `self.current height` (- (`self.current height`) (`self.story height`)))
            (set `self.ismovement` false)))))))

(event `openliftdoors`
  (set `self.Doorlocation1` (`SceneComponent.K2_GetComponentLocation` (`self.Lift_Door2_StaticMesh`)))
  (set `self.doorlocation2` (`SceneComponent.K2_GetComponentLocation` (`self.Lift_Door3_StaticMesh`)))
  (set `self.doorstop` false)
  (bind (_direction _newtrack_0 _newtrack2) (`Timeline|Timeline_0` :!label _label)
    (:`Update`
      (`SceneComponent.K2_SetWorldLocation` (`self.Lift_Door2_StaticMesh`) (+ _newtrack_0 (`self.Doorlocation1`)) false false)
      (`SceneComponent.K2_SetWorldLocation` (`self.Lift_Door3_StaticMesh`) (+ _newtrack2 (`self.doorlocation2`)) false false)
      (set `self.doorstop` true))))

(event `self.doorclosetrigger.OnComponentBeginOverlap`
  (params (OverlappedComponent :type "PrimitiveComponent Object Reference") (OtherActor :type "Actor Object Reference") (OtherComp :type "PrimitiveComponent Object Reference") (OtherBodyIndex :type Integer) (bFromSweep :type Boolean) (SweepResult :type "HitResult Structure (by ref)")))

(event `closeliftdoors`
  (set `self.doorstop` false)
  (goto _label :!via `Reverse`))

(event `self.leveltriggertop.OnComponentBeginOverlap`
  (params (OverlappedComponent :type "PrimitiveComponent Object Reference") (OtherActor :type "Actor Object Reference") (OtherComp :type "PrimitiveComponent Object Reference") (OtherBodyIndex :type Integer) (bFromSweep :type Boolean) (SweepResult :type "HitResult Structure (by ref)")))

(event `self.leveltriggerbottom.OnComponentBeginOverlap`
  (params (OverlappedComponent :type "PrimitiveComponent Object Reference") (OtherActor :type "Actor Object Reference") (OtherComp :type "PrimitiveComponent Object Reference") (OtherBodyIndex :type Integer) (bFromSweep :type Boolean) (SweepResult :type "HitResult Structure (by ref)")))

(fn `UserConstructionScript`)